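; Puppeteer manager actor that drives a MetaHuman's face from Live Link ARKit blendshapes with per-shape calibration.
; Each tick it reads raw curve values, zeroing disabled shapes, normalises them to stored min/max ranges and passes them to the Face AnimBP.
; An optional calibration widget shows live values and triggers neutral capture, min/max setting, resets, enable toggles and save/load of ranges via SaveGame slots.
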(event `self.ReceiveBeginPlay`
  (bind _calibration_ui (`self.Calibration_UI`))
  (if (`self.isPuppeteerEnabled`)
    ;[1 1 1] Check Metahuman Ref has been set
    (if (`KismetSystemLibrary.IsValid` (`self.Metahuman_Ref`))
      (`|ExecutionSequence`
        (:`then_0`
          ;[1 1 1] Create Calibration Widget
          (bind _returnvalue (`|CreateWidget` "/Puppeteer/Blueprints/UI/Puppeteer_Calibration_UI.Puppeteer_Calibration_UI_C" (`GameplayStatics.GetPlayerController` 0)))
          (set `self.Calibration_UI` _returnvalue)
          ;[1 0.9153 0] Show Calibration UI
          ; - Should be toggleable
          (if (`self.isUIEnabled`)
            (`UserWidget.AddToViewport` _calibration_ui 0)
            (`Widget.SetVisibility` _calibration_ui "Visible")
            ;[1 1 1] Bind events
            (`self.BindUIEvents`)))
        (:`then_1`
          ;[1 1 1] Initialise the calibration value maps to a default value
          (bind _enumvalue (foreach `/Puppeteer/Enums/AppleARKitBlendshapes` false)
            (:`LoopBody`
              (`BlueprintMapLibrary.Map_Add` (`self.ARKit_BS_Min`) _enumvalue)
              (`BlueprintMapLibrary.Map_Add` (`self.ARKit_BS_Max`) _enumvalue 1.0)
              (`BlueprintMapLibrary.Map_Add` (`self.ARKit_BS_isEnabled`) _enumvalue true))))
        (:`then_2`
          ;[1 1 1] Get reference to Face Skeletal Mesh and AnimBP
          (for _array_element (`self.K2_GetComponentsByClass` (`self.Metahuman_Ref`) "/Script/Engine.SkeletalMeshComponent")
            (if (== (`KismetSystemLibrary.GetDisplayName` _array_element) "Face")
              (bind _output_get (set `self.FaceSkeletalMesh` _array_element))
              (set `self.FaceAnimInstance` (`SkeletalMeshComponent.GetAnimInstance` _output_get))))))
      (else
        (`KismetSystemLibrary.PrintString` "Error: Metahuman BP reference has not been set in Puppeteer Manager. Puppeteer is disabled.")))))

(event `self.ReceiveTick`
  (params (DeltaSeconds :type "Float (single-precision)"))
  (`|ExecutionSequence`
    (:`then_0`
      ;[1 1 1] Evaluate Live Link frame and add raw values to a map
      (bind _dataresult (`|EvaluateLiveLinkFrameWithSpecificRole` (`self.LiveLinkSubject`) "/Script/LiveLinkInterface.LiveLinkBasicRole")
        (:`then`
          (bind _enumvalue (foreach `/Puppeteer/Enums/AppleARKitBlendshapes` false)
            (:`LoopBody`
              (`BlueprintMapLibrary.Map_Add` (`self.ARKit_BS_RawValues`) _enumvalue (select `bool` (`BlueprintMapLibrary.Map_Find` (`self.ARKit_BS_isEnabled`) _enumvalue) :`true` (`LiveLinkBlueprintLibrary.GetPropertyValue` _dataresult (`KismetStringLibrary.Conv_StringToName` (`|GetEnumeratorNameAsString` _enumvalue))) :!type "Float (double-precision)")))))))
    (:`then_1`
      ;[1 1 1] Take the raw data and normalise it to a calibrated range.
      (`self.Normalise Values`))
    (:`then_2`
      ;[1 1 1] Update Anim Instance with latest normalised values
      (message `/Puppeteer/Blueprints/Puppeteer_AnimBP_Interface.UpdateARKitValues` (`self.FaceAnimInstance`) (`self.ARKit BS_NormalisedValues`)))
    (:`then_3`
      ;[1 1 1] Update Calibration UI with latest values
      (if (`self.isUIEnabled`)
        (bind _enumvalue_2 (foreach `/Puppeteer/Enums/AppleARKitBlendshapes` false)
          (:`LoopBody`
            (message `/Puppeteer/Blueprints/UI/Calibration_UI_Interface.UpdateARKitBSState` (`self.Calibration_UI`) _enumvalue_2 (`BlueprintMapLibrary.Map_Find` (`self.ARKit_BS_isEnabled`) _enumvalue_2) (`BlueprintMapLibrary.Map_Find` (`self.ARKit_BS_RawValues`) _enumvalue_2) (`BlueprintMapLibrary.Map_Find` (`self.ARKit_BS_Min`) _enumvalue_2) (`BlueprintMapLibrary.Map_Find` (`self.ARKit_BS_Max`) _enumvalue_2))))))))

(fn `BindUIEvents`
  (bind _calibration_ui (`self.Calibration_UI`))
  (bind _calibration_ui_2 (`self.Calibration_UI`))
  (`|ExecutionSequence`
    (:`then_0`
      ;[1 1 1] Calibration UI events
      (add `/Puppeteer/Blueprints/UI/Puppeteer_Calibration_UI.SaveCalibration` _calibration_ui_2 (`|CreateDelegate` :!event `SaveCalibration`))
      (add `/Puppeteer/Blueprints/UI/Puppeteer_Calibration_UI.LoadCalibration` _calibration_ui_2 (`|CreateDelegate` :!event `LoadCalibration`))
      (add `/Puppeteer/Blueprints/UI/Puppeteer_Calibration_UI.SetNeutral` _calibration_ui_2 (`|CreateDelegate` :!event `Set Current Values as Min`))
      (add `/Puppeteer/Blueprints/UI/Puppeteer_Calibration_UI.ResetCalibration` _calibration_ui_2 (`|CreateDelegate` :!event `ResetCalibration`))
      (add `/Puppeteer/Blueprints/UI/Puppeteer_Calibration_UI.DisableAllARKitBS` _calibration_ui_2 (`|CreateDelegate` :!event `DisableAllARKitBS`))
      (add `/Puppeteer/Blueprints/UI/Puppeteer_Calibration_UI.EnableAllARKitBS` _calibration_ui_2 (`|CreateDelegate` :!event `EnableAllARKitBS`)))
    (:`then_1`
      ;[1 1 1] Calibration UI events for Single ARKitBS
      (add `/Puppeteer/Blueprints/UI/Puppeteer_Calibration_UI.didSetMaxForARKitBS` _calibration_ui (`|CreateDelegate` :!event `SetMaxForARKitBS`))
      (add `/Puppeteer/Blueprints/UI/Puppeteer_Calibration_UI.didSetMinForARKitBS` _calibration_ui (`|CreateDelegate` :!event `SetMinForARKitBS`))
      (add `/Puppeteer/Blueprints/UI/Puppeteer_Calibration_UI.ResetCalibrationForARKitBS` _calibration_ui (`|CreateDelegate` :!event `ResetCalibrationForARKitBS`))
      (add `/Puppeteer/Blueprints/UI/Puppeteer_Calibration_UI.SetEnabledForARKitBS` _calibration_ui (`|CreateDelegate` :!event `SetEnabledForARKitBS`)))))

(fn `DisableAllARKitBS`
  (bind _enumvalue (foreach `/Puppeteer/Enums/AppleARKitBlendshapes` false)
    (:`LoopBody`
      (`BlueprintMapLibrary.Map_Add` (`self.ARKit_BS_isEnabled`) _enumvalue))))

(fn `EnableAllARKitBS`
  (bind _enumvalue (foreach `/Puppeteer/Enums/AppleARKitBlendshapes` false)
    (:`LoopBody`
      (`BlueprintMapLibrary.Map_Add` (`self.ARKit_BS_isEnabled`) _enumvalue true))))

(fn `LoadCalibration`
  (params (CalibrationName :type Name))
  (bind _returnvalue (`GameplayStatics.LoadGameFromSlot` (`KismetStringLibrary.Conv_NameToString` CalibrationName)))
  (bind _ascalibration_save (cast `/Puppeteer/Blueprints/Calibration_Save` _returnvalue)
    (:`then`
      (set `self.ARKit_BS_Max` (`/Puppeteer/Blueprints/Calibration_Save.ARKit_BS_Max` _ascalibration_save))
      (set `self.ARKit_BS_Min` (`/Puppeteer/Blueprints/Calibration_Save.ARKit_BS_Min` _ascalibration_save)))
    (:`CastFailed`
      (`KismetSystemLibrary.PrintString` "Failed to load calibration: Could not cast to Calibration_Save"))))

(fn `Normalise Values`
  (locals (CurrentARKitBS :type "/Puppeteer/Enums/AppleARKitBlendshapes Enum") (RawValue :type "Float (double-precision)") (Min :type "Float (double-precision)") (Max :type "Float (double-precision)"))
  (bind _currentarkitbs (`local.CurrentARKitBS`))
  (bind _keys (`BlueprintMapLibrary.Map_Keys` (`self.ARKit_BS_RawValues`)))
  (for _array_element _keys
    (set `local.CurrentARKitBS` _array_element)
    (`|ExecutionSequence`
      (:`then_0`
        ;[1 1 1] Get the values
        (set `local.RawValue` (`BlueprintMapLibrary.Map_Find` (`self.ARKit_BS_RawValues`) _currentarkitbs))
        (set `local.Min` (`BlueprintMapLibrary.Map_Find` (`self.ARKit_BS_Min`) _currentarkitbs))
        (set `local.Max` (`BlueprintMapLibrary.Map_Find` (`self.ARKit_BS_Max`) _currentarkitbs)))
      (:`then_1`
        ;[1 1 1] Normalise the value based on the min/max range
        (`BlueprintMapLibrary.Map_Add` (`self.ARKit BS_NormalisedValues`) (`local.CurrentARKitBS`) (`KismetMathLibrary.NormalizeToRange` (`local.RawValue`) (`local.Min`) (`local.Max`)))))))

(fn `ResetCalibration`
  (bind _enumvalue (foreach `/Puppeteer/Enums/AppleARKitBlendshapes` false)
    (:`LoopBody`
      (`BlueprintMapLibrary.Map_Add` (`self.ARKit_BS_Min`) _enumvalue)
      (`BlueprintMapLibrary.Map_Add` (`self.ARKit_BS_Max`) _enumvalue 1.0))))

(fn `ResetCalibrationForARKitBS`
  (params (ARKitBS :type "/Puppeteer/Enums/AppleARKitBlendshapes Enum" :default "NewEnumerator0"))
  (`BlueprintMapLibrary.Map_Add` (`self.ARKit_BS_Min`) ARKitBS)
  (`BlueprintMapLibrary.Map_Add` (`self.ARKit_BS_Max`) ARKitBS 1.0))

(fn `SaveCalibration`
  (params (CalibrationName :type Name))
  (bind _returnvalue (`GameplayStatics.CreateSaveGameObject` "/Puppeteer/Blueprints/Calibration_Save.Calibration_Save_C"))
  (set `/Puppeteer/Blueprints/Calibration_Save.ARKit_BS_Max` (`self.ARKit_BS_Max`) _returnvalue)
  (set `/Puppeteer/Blueprints/Calibration_Save.ARKit_BS_Min` (`self.ARKit_BS_Min`) _returnvalue)
  (`GameplayStatics.SaveGameToSlot` _returnvalue (`KismetStringLibrary.Conv_NameToString` (`local.CalibrationName`))))

(fn `Set Current Values as Min`
  ;[1 1 1] Take all the current raw values and set them as the min for that blendshape, effectively setting what the rig control values should be when your face is neutral
  (bind _enumvalue (foreach `/Puppeteer/Enums/AppleARKitBlendshapes` false)
    (:`LoopBody`
      (`BlueprintMapLibrary.Map_Add` (`self.ARKit_BS_Min`) _enumvalue (`BlueprintMapLibrary.Map_Find` (`self.ARKit_BS_RawValues`) _enumvalue)))))

(fn `SetEnabledForARKitBS`
  (params (isEnabled :type Boolean) (ARKitBS :type "/Puppeteer/Enums/AppleARKitBlendshapes Enum" :default "NewEnumerator0"))
  (`BlueprintMapLibrary.Map_Add` (`self.ARKit_BS_isEnabled`) ARKitBS isEnabled))

(fn `SetMaxForARKitBS`
  (params (ARKitBS :type "/Puppeteer/Enums/AppleARKitBlendshapes Enum" :default "NewEnumerator0"))
  (`BlueprintMapLibrary.Map_Add` (`self.ARKit_BS_Max`) ARKitBS (`BlueprintMapLibrary.Map_Find` (`self.ARKit_BS_RawValues`) ARKitBS)))

(fn `SetMinForARKitBS`
  (params (ARKitBS :type "/Puppeteer/Enums/AppleARKitBlendshapes Enum" :default "NewEnumerator0"))
  (`BlueprintMapLibrary.Map_Add` (`self.ARKit_BS_Min`) ARKitBS (`BlueprintMapLibrary.Map_Find` (`self.ARKit_BS_RawValues`) ARKitBS)))

(fn `UserConstructionScript`)