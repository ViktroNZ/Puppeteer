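; User_BP is a user Blueprint that toggles the Calibration_UI widget on screen with the 1 key.
; The first press creates the widget once for player 0, stores it and adds it to the viewport.
; Each press then runs a FlipFlop on the stored widget, alternating it between visible and hidden, starting with visible.
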(event `Key|One`
  (params (Key :type "Key Structure"))
  (bind _calibration_ui (`self.Calibration_UI`))
  (:`Pressed`
    (`|ExecutionSequence`
      (:`then_0`
        (`/Engine/EditorBlueprintResources/StandardMacros.DoOnce` false
          (:`Completed`
            (bind _returnvalue (`|CreateWidget` "/Puppeteer/UI/Calibration_UI.Calibration_UI_C" (`GameplayStatics.GetPlayerController` 0)))
            (bind _output_get (set `self.Calibration_UI` _returnvalue))
            (`UserWidget.AddToViewport` _output_get 0))))
      (:`then_1`
        (if (`KismetSystemLibrary.IsValid` (`self.Calibration_UI`))
          (`/Engine/EditorBlueprintResources/StandardMacros.FlipFlop`
            (:`A`
              (`Widget.SetVisibility` _calibration_ui "Visible"))
            (:`B`
              (`Widget.SetVisibility` _calibration_ui "Hidden"))))))))

(fn `UserConstructionScript`)