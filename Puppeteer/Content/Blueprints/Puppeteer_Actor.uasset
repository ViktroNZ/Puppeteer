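; Puppeteer actor that spawns a MetaHuman and drives its face from Live Link ARKit blendshape data.
; On BeginPlay it fills per-blendshape calibration maps and assigns the Puppeteer AnimBP to the Face mesh.
; Each tick it reads the Live Link frame, zeroes disabled shapes, normalises values to their min/max and sends them to the AnimBP.
; Optional autocalibration widens ranges from incoming values, with functions for manual setting and reset.
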(event `self.ReceiveBeginPlay`
  (`|ExecutionSequence`
    (:`then_0`
      ;[1 1 1] Spawn the Metahuman
      (bind _returnvalue (`|SpawnActorFromClass` (`self.MetahumanActorClass`) (`KismetMathLibrary.MakeTransform` (0.0 0.0 0.0) (struct :`Yaw` 90.0)) "Undefined" "OverrideRootScale" null null))
      (set `self.MetahumanActor` _returnvalue))
    (:`then_1`
      ;[1 1 1] Initialise the calibration value maps to a default value
      (bind _enumvalue (foreach `/Puppeteer/Enums/AppleARKitBlendshapes` false)
        (:`LoopBody`
          (`self.SetMinMaxForHeadRotations` _enumvalue)
          (`BlueprintMapLibrary.Map_Add` (`self.ARKit_BS_Min`) _enumvalue)
          (`BlueprintMapLibrary.Map_Add` (`self.ARKit_BS_Max`) _enumvalue 1.0)
          (`BlueprintMapLibrary.Map_Add` (`self.ARKit_BS_isEnabled`) _enumvalue true))))
    (:`then_2`
      ;[1 1 1] Get a reference to the Metahuman AnimBP
      (for _array_element (`self.K2_GetComponentsByClass` (`self.MetahumanActor`) "/Script/Engine.SkeletalMeshComponent")
        (if (`KismetStringLibrary.Contains` (`KismetSystemLibrary.GetDisplayName` _array_element) "Face")
          (`SkeletalMeshComponent.SetAnimInstanceClass` _array_element "/Puppeteer/Blueprints/Puppeteer_AnimBP.Puppeteer_AnimBP_C")
          (set `self.Metahuman_AnimBP` (`SkeletalMeshComponent.GetAnimInstance` _array_element)))))))

(event `self.ReceiveTick`
  (params (DeltaSeconds :type "Float (single-precision)"))
  (`|ExecutionSequence`
    (:`then_0`
      ;[1 1 1] Evaluate Live Link frame and add raw values to a map
      (bind _dataresult (`|EvaluateLiveLinkFrameWithSpecificRole` (`self.LiveLinkSubject`) "/Script/LiveLinkInterface.LiveLinkBasicRole")
        (:`then`
          (bind _enumvalue (foreach `/Puppeteer/Enums/AppleARKitBlendshapes` false)
            (:`LoopBody`
              (`BlueprintMapLibrary.Map_Add` (`self.ARKit_BS_RawValues`) _enumvalue (select `bool` (`BlueprintMapLibrary.Map_Find` (`self.ARKit_BS_isEnabled`) _enumvalue) :`true` (`LiveLinkBlueprintLibrary.GetPropertyValue` _dataresult (`KismetStringLibrary.Conv_StringToName` (`|GetEnumeratorNameAsString` _enumvalue))))))))))
    (:`then_1`
      ;[1 1 1] Take the raw data and normalise it to a calibrated range. Autocalibrate the range if autocalibration is enabled
      (`self.Normalise and Autocalibrate Values`))
    (:`then_2`
      ;[1 1 1] Pass ARKit values to Anim BP
      (message `/Puppeteer/Blueprints/MH_Puppeteer_Interface.UpdateARKitBSValues` (`self.Metahuman_AnimBP`) (`self.ARKit_BS_NormalisedValues`)))))

(fn `Normalise and Autocalibrate Values`
  (locals (RawValue :type "Float (double-precision)") (Min :type "Float (double-precision)") (Max :type "Float (double-precision)") (CurrentARKitBS :type "/Puppeteer/Enums/AppleARKitBlendshapes Enum"))
  (bind _rawvalue (`local.RawValue`))
  (bind _currentarkitbs (`local.CurrentARKitBS`))
  (bind _currentarkitbs_2 (`local.CurrentARKitBS`))
  (bind _keys (`BlueprintMapLibrary.Map_Keys` (`self.ARKit_BS_RawValues`)))
  (for _array_element _keys
    (set `local.CurrentARKitBS` _array_element)
    (`|ExecutionSequence`
      (:`then_0`
        ;[1 1 1] Get the values
        (set `local.RawValue` (`BlueprintMapLibrary.Map_Find` (`self.ARKit_BS_RawValues`) _currentarkitbs))
        (set `local.Min` (`BlueprintMapLibrary.Map_Find` (`self.ARKit_BS_Min`) _currentarkitbs))
        (set `local.Max` (`BlueprintMapLibrary.Map_Find` (`self.ARKit_BS_Max`) _currentarkitbs)))
      (:`then_1`
        ;[1 1 1] Auto calibrate the range of min and max depending on whether the raw value is greater or smaller than min/max
        (if (`self.isAutocalibrateEnabled`)
          (`|ExecutionSequence`
            (:`then_0`
              (if (< (`local.RawValue`) (`local.Min`))
                (`BlueprintMapLibrary.Map_Add` (`self.ARKit_BS_Min`) _currentarkitbs_2 _rawvalue)))
            (:`then_1`
              (if (> (`local.RawValue`) (`local.Max`))
                (`BlueprintMapLibrary.Map_Add` (`self.ARKit_BS_Max`) _currentarkitbs_2 _rawvalue))))))
      (:`then_2`
        ;[1 1 1] Normalise the value based on the min/max range
        (`BlueprintMapLibrary.Map_Add` (`self.ARKit_BS_NormalisedValues`) (`local.CurrentARKitBS`) (`KismetMathLibrary.NormalizeToRange` (`local.RawValue`) (`local.Min`) (`local.Max`)))))))

(fn `ResetCalibration`
  (bind _enumvalue (foreach `/Puppeteer/Enums/AppleARKitBlendshapes` false)
    (:`LoopBody`
      (`BlueprintMapLibrary.Map_Add` (`self.ARKit_BS_Min`) _enumvalue 1.0)
      (`BlueprintMapLibrary.Map_Add` (`self.ARKit_BS_Max`) _enumvalue))))

(fn `SetMaxForARKitBS`
  (params (forBlendshape :type "/Puppeteer/Enums/AppleARKitBlendshapes Enum" :default "NewEnumerator0"))
  (`BlueprintMapLibrary.Map_Add` (`self.ARKit_BS_Max`) forBlendshape (`BlueprintMapLibrary.Map_Find` (`self.ARKit_BS_RawValues`) forBlendshape)))

(fn `SetMinForARKitBS`
  (params (forBlendshape :type "/Puppeteer/Enums/AppleARKitBlendshapes Enum" :default "NewEnumerator0"))
  (`BlueprintMapLibrary.Map_Add` (`self.ARKit_BS_Min`) forBlendshape (`BlueprintMapLibrary.Map_Find` (`self.ARKit_BS_RawValues`) forBlendshape)))

(fn `SetMinMaxForHeadRotations`
  (params (currentARKitBS :type "/Puppeteer/Enums/AppleARKitBlendshapes Enum" :default "NewEnumerator0"))
  (bind _headrotationanglemax (`self.HeadRotationAngleMax`))
  (bind _currentarkitbs (`local.currentARKitBS`))
  (switch `/Puppeteer/Enums/AppleARKitBlendshapes` currentARKitBS
    (:`NewEnumerator52`
      _)
    (:`NewEnumerator53`
      _)
    (:`NewEnumerator54`
      _))
  (`BlueprintMapLibrary.Map_Add` (`self.ARKit_BS_Max`) _currentarkitbs _headrotationanglemax)
  (`BlueprintMapLibrary.Map_Add` (`self.ARKit_BS_Min`) _currentarkitbs (* _headrotationanglemax -1.0)))

(fn `UserConstructionScript`)