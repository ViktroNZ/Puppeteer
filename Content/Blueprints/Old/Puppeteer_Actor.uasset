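; Puppeteer actor that spawns a MetaHuman on BeginPlay and holds calibration logic for ARKit face blendshape values.
; Raw values are normalised against per-blendshape min/max maps, which optionally widen automatically when a value falls outside them.
; Helpers capture the current raw value as min or max, or reset ranges inverted for recalibration.
; Tick is empty, nothing here calls the calibration functions, and the head-rotation range function is an unfinished switch.
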(event `self.ReceiveBeginPlay`
  (`|ExecutionSequence`
    (:`then_0`
      ;[1 1 1] Spawn the Metahuman
      (bind _returnvalue (`|SpawnActorFromClass` (`self.MetahumanActorClass`) (`KismetMathLibrary.MakeTransform` (0.0 0.0 0.0) (struct :`Yaw` 90.0)) "Undefined" "SelectDefaultAtRuntime" null null))
      (set `self.MetahumanActor` _returnvalue))))

(event `self.ReceiveTick`
  (params (DeltaSeconds :type "Float (single-precision)"))
  (`|ExecutionSequence`))

(fn `Normalise and Autocalibrate Values`
  (locals (RawValue :type "Float (double-precision)") (Min :type "Float (double-precision)") (Max :type "Float (double-precision)") (CurrentARKitBS :type "/Puppeteer/Enums/AppleARKitBlendshapes Enum"))
  (bind _rawvalue (`local.RawValue`))
  (bind _currentarkitbs (`local.CurrentARKitBS`))
  (bind _currentarkitbs_2 (`local.CurrentARKitBS`))
  (bind _keys (`BlueprintMapLibrary.Map_Keys` (`self.ARKit_BS_RawValues`)))
  (for _array_element _keys
    (set `local.CurrentARKitBS` _array_element)
    (`|ExecutionSequence`
      (:`then_0`
        ;[1 1 1] Get the values
        (set `local.RawValue` (`BlueprintMapLibrary.Map_Find` (`self.ARKit_BS_RawValues`) _currentarkitbs))
        (set `local.Min` (`BlueprintMapLibrary.Map_Find` (`self.ARKit_BS_Min`) _currentarkitbs))
        (set `local.Max` (`BlueprintMapLibrary.Map_Find` (`self.ARKit_BS_Max`) _currentarkitbs)))
      (:`then_1`
        ;[1 1 1] Auto calibrate the range of min and max depending on whether the raw value is greater or smaller than min/max
        (if (`self.isAutocalibrateEnabled`)
          (`|ExecutionSequence`
            (:`then_0`
              (if (< (`local.RawValue`) (`local.Min`))
                (`BlueprintMapLibrary.Map_Add` (`self.ARKit_BS_Min`) _currentarkitbs_2 _rawvalue)))
            (:`then_1`
              (if (> (`local.RawValue`) (`local.Max`))
                (`BlueprintMapLibrary.Map_Add` (`self.ARKit_BS_Max`) _currentarkitbs_2 _rawvalue))))))
      (:`then_2`
        ;[1 1 1] Normalise the value based on the min/max range
        (`BlueprintMapLibrary.Map_Add` (`self.ARKit_BS_NormalisedValues`) (`local.CurrentARKitBS`) (`KismetMathLibrary.NormalizeToRange` (`local.RawValue`) (`local.Min`) (`local.Max`)))))))

(fn `ResetCalibration`
  (bind _enumvalue (foreach `/Puppeteer/Enums/AppleARKitBlendshapes` false)
    (:`LoopBody`
      (`BlueprintMapLibrary.Map_Add` (`self.ARKit_BS_Min`) _enumvalue 1.0)
      (`BlueprintMapLibrary.Map_Add` (`self.ARKit_BS_Max`) _enumvalue))))

(fn `SetMaxForARKitBS`
  (params (forBlendshape :type "/Puppeteer/Enums/AppleARKitBlendshapes Enum" :default "NewEnumerator0"))
  (`BlueprintMapLibrary.Map_Add` (`self.ARKit_BS_Max`) forBlendshape (`BlueprintMapLibrary.Map_Find` (`self.ARKit_BS_RawValues`) forBlendshape)))

(fn `SetMinForARKitBS`
  (params (forBlendshape :type "/Puppeteer/Enums/AppleARKitBlendshapes Enum" :default "NewEnumerator0"))
  (`BlueprintMapLibrary.Map_Add` (`self.ARKit_BS_Min`) forBlendshape (`BlueprintMapLibrary.Map_Find` (`self.ARKit_BS_RawValues`) forBlendshape)))

(fn `SetMinMaxForHeadRotations`
  (params (currentARKitBS :type "/Puppeteer/Enums/AppleARKitBlendshapes Enum" :default "NewEnumerator0"))
  (switch `/Puppeteer/Enums/AppleARKitBlendshapes` currentARKitBS))

(fn `UserConstructionScript`)